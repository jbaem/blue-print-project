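; BP_FallingPlate is an environment platform that sinks while an actor overlaps it and rises back to its start position afterwards.
; It records its location on BeginPlay, and begin and end overlap events toggle an overlap flag.
; Tick moves it along Z at FallingSpeed scaled by delta time, with no lower limit on descent and upward movement only while below the start height.
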(event `self.ReceiveBeginPlay`
  (set `self.DefaultPosition` (`self.K2_GetActorLocation`)))

(event `self.ReceiveTick`
  (params (DeltaSeconds :type "Float (single-precision)"))
  (bind (_returnvalue_x _returnvalue_y _returnvalue_z) (`KismetMathLibrary.BreakVector` (`self.K2_GetActorLocation`)))
  (bind (_returnvalue_x_2 _returnvalue_y_2 _returnvalue_z_2) (`KismetMathLibrary.BreakVector` (`self.K2_GetActorLocation`)))
  (bind (_defaultposition_x _defaultposition_y _defaultposition_z) (`KismetMathLibrary.BreakVector` (`self.DefaultPosition`)))
  (if (`self.IsOverlaped`)
    (`self.K2_SetActorLocation` (`KismetMathLibrary.MakeVector` _returnvalue_x _returnvalue_y (+ _returnvalue_z (* DeltaSeconds (* (`self.FallingSpeed`) -1.0)))))
    (elif (< _returnvalue_z_2 _defaultposition_z)
      (`self.K2_SetActorLocation` (`KismetMathLibrary.MakeVector` _returnvalue_x_2 _returnvalue_y_2 (+ _returnvalue_z_2 (* DeltaSeconds (`self.FallingSpeed`))))))))

(event `self.ReceiveActorBeginOverlap`
  (params (OtherActor :type "Actor Object Reference"))
  (set `self.IsOverlaped` true))

(event `self.ReceiveActorEndOverlap`
  (params (OtherActor :type "Actor Object Reference"))
  (set `self.IsOverlaped` false))

(fn `UserConstructionScript`)