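; Jump pad that springs up when an actor overlaps it and launches player characters into the air.
; A timeline moves the plate along its relative Z by PopLength, while IsPrepared blocks retriggering until the animation finishes.
; Any valid actor triggers the pop, but only BP_DefaultCharacter is launched, along the pad's up vector scaled by PopPower with vertical velocity overridden.
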(event `self.ReceiveActorBeginOverlap`
  (params (OtherActor :type "Actor Object Reference"))
  (`/Engine/EditorBlueprintResources/StandardMacros.IsValid` OtherActor
    (:`Is Valid`
      (if (`self.IsPrepared`)
        (`|ExecutionSequence`
          (:`then_0`
            (set `self.IsPrepared` false)
            (bind (_direction _poprate) (`Timeline|타임라인` :!via `PlayFromStart`)
              (:`Update`
                (`SceneComponent.K2_SetRelativeLocation` (`self.Plate`) (`KismetMathLibrary.MakeVector` 0.0 0.0 (* _poprate (`self.PopLength`))) false false))
              (:`Finished`
                (set `self.IsPrepared` true))))
          (:`then_1`
            (bind _asbp_default_character (cast `/Game/Characters/Robot/BP_DefaultCharacter` OtherActor))
            (`Character.LaunchCharacter` _asbp_default_character (* (`self.GetActorUpVector`) (`self.PopPower`)) false true)))))))

(fn `UserConstructionScript`)