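; BP_StartPoint is a start point Blueprint whose Ring component rises and spins when used.
; The Use event waits through a short delay, then plays the TL_Use timeline from the start.
; Timeline curves, scaled by Height and RoundDegree, drive the ring's relative Z location and yaw.
; BeginPlay stores the actor's location in DefaultPosition, which the graphs shown here never read.
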(event `self.ReceiveBeginPlay`
  (set `self.DefaultPosition` (`self.K2_GetActorLocation`)))

(event `Use`
  (`KismetSystemLibrary.Delay` 2.0)
  (bind (_direction _heightrate _rotaterate) (`Timeline|TL_Use` :!via `PlayFromStart`)
    (:`Update`
      (`SceneComponent.K2_SetRelativeLocation` (`self.Ring`) (`KismetMathLibrary.MakeVector` 0.0 0.0 (* _heightrate (`self.Height`))) false false)
      (`SceneComponent.K2_SetRelativeRotation` (`self.Ring`) (`KismetMathLibrary.MakeRotator` 0.0 0.0 (* _rotaterate (`self.RoundDegree`))) false false))))

(fn `UserConstructionScript`)