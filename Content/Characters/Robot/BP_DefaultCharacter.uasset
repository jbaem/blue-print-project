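; Player character Blueprint with Enhanced Input movement, adjustable camera speed, running, multi-jump and position reset.
; Run switches max walk speed, while jumps use a DoN-gated launch whose limit GetJumpItem raises and landing restores to default.
; Tick flags fast falls so landing triggers FallDown, which plays a montage and blocks moving and jumping until a delay after it completes.
; Reset returns to BasePosition, triggers FallDown and calls Use on BP_StartPoint.
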(event `self.ReceiveBeginPlay`
  (set `CharacterMovementComponent.MaxWalkSpeed` (`self.WalkSpeed`) (`self.CharacterMovement`))
  (set `self.TotalJumpCount` (`self.DefaultJumpCount`)))

(event `self.ReceiveControllerChanged`
  (params (OldController :type "Controller Object Reference") (NewController :type "Controller Object Reference"))
  (bind `_as플레이어_컨트롤러` (cast `PlayerController` NewController))
  (`EnhancedInputSubsystemInterface.AddMappingContext` (pcsubsystem `EnhancedInputLocalPlayerSubsystem` `_as플레이어_컨트롤러`) (`self.Mapping Context`) 0 (struct)))

(event `EnhancedInput|/Game/Inputs/Actions/IA_Look`
  (params (ActionValue :type "Vector2D Structure") (ElapsedSeconds :type "Float (double-precision)") (TriggeredSeconds :type "Float (double-precision)") (InputAction :type "InputAction Object Reference" :default "/Game/Inputs/Actions/IA_Look.IA_Look"))
  (bind _cameraspeedrate (`self.CameraSpeedRate`))
  (:`Triggered`
    (`self.AddControllerYawInput` (* ActionValue_X _cameraspeedrate))
    (`self.AddControllerPitchInput` (* ActionValue_Y _cameraspeedrate))))

(event `EnhancedInput|/Game/Inputs/Actions/IA_ControlCameraSpeed`
  (params (ActionValue :type "Float (double-precision)") (ElapsedSeconds :type "Float (double-precision)") (TriggeredSeconds :type "Float (double-precision)") (InputAction :type "InputAction Object Reference" :default "/Game/Inputs/Actions/IA_ControlCameraSpeed.IA_ControlCameraSpeed"))
  (bind _returnvalue (`KismetMathLibrary.FClamp` (+ (* ActionValue 0.05) (`self.CameraSpeedRate`)) 0.05))
  (:`Triggered`
    (set `self.CameraSpeedRate` _returnvalue)
    (`KismetSystemLibrary.PrintString` (`KismetStringLibrary.BuildString_Double` "" "Camera Rotate Speed : " _returnvalue))))

(event `EnhancedInput|/Game/Inputs/Actions/IA_Move`
  (params (ActionValue :type "Vector2D Structure") (ElapsedSeconds :type "Float (double-precision)") (TriggeredSeconds :type "Float (double-precision)") (InputAction :type "InputAction Object Reference" :default "/Game/Inputs/Actions/IA_Move.IA_Move"))
  (bind (_returnvalue_roll _returnvalue_pitch _returnvalue_yaw) (`KismetMathLibrary.BreakRotator` (`self.GetControlRotation`)))
  (bind (_returnvalue_roll_2 _returnvalue_pitch_2 _returnvalue_yaw_2) (`KismetMathLibrary.BreakRotator` (`self.GetControlRotation`)))
  (:`Triggered`
    (if (`self.CanMove`)
      (`|ExecutionSequence`
        (:`then_0`
          (`self.AddMovementInput` (`KismetMathLibrary.GetRightVector` (`KismetMathLibrary.MakeRotator` _returnvalue_roll_2 0.0 _returnvalue_yaw_2)) ActionValue_X))
        (:`then_1`
          (`self.AddMovementInput` (`KismetMathLibrary.GetForwardVector` (`KismetMathLibrary.MakeRotator` 0.0 0.0 _returnvalue_yaw)) ActionValue_Y))))))

(event `EnhancedInput|/Game/Inputs/Actions/IA_Run`
  (params (ActionValue :type Boolean) (ElapsedSeconds :type "Float (double-precision)") (TriggeredSeconds :type "Float (double-precision)") (InputAction :type "InputAction Object Reference" :default "/Game/Inputs/Actions/IA_Run.IA_Run"))
  (:`Started`
    (`self.RunActive`))
  (:`Completed`
    (`self.RunDeactive`)))

(event `RunActive`
  (if (not (`self.IsRunning`))
    (set `CharacterMovementComponent.MaxWalkSpeed` (`self.RunSpeed`) (`self.CharacterMovement`))
    (set `self.IsRunning` true)))

(event `RunDeactive`
  (set `CharacterMovementComponent.MaxWalkSpeed` (`self.WalkSpeed`) (`self.CharacterMovement`))
  (set `self.IsRunning` false))

(event `EnhancedInput|/Game/Inputs/Actions/IA_Jump`
  (params (ActionValue :type Boolean) (ElapsedSeconds :type "Float (double-precision)") (TriggeredSeconds :type "Float (double-precision)") (InputAction :type "InputAction Object Reference" :default "/Game/Inputs/Actions/IA_Jump.IA_Jump"))
  (:`Started`
    (if (`self.CanMove`)
      (`/Engine/EditorBlueprintResources/StandardMacros.Do N` (`self.TotalJumpCount`) :!label _label
        (:`Exit`
          (`self.LaunchCharacter` (0.0 0.0 420.0) false true)))))
  (:`Completed`
    (`self.StopJumping`)))

(event `self.OnLanded`
  (params (Hit :type "HitResult Structure (by ref)"))
  (`|ExecutionSequence`
    (:`then_0`
      (goto _label :!via `Reset`))
    (:`then_1`
      (set `self.TotalJumpCount` (`self.DefaultJumpCount`)))
    (:`then_2`
      (if (`self.WillFallDown`)
        (`self.FallDown`)))))

(event `GetJumpItem`
  (set `self.TotalJumpCount` (+ (`self.TotalJumpCount`) 1)))

(event `self.ReceiveTick`
  (params (DeltaSeconds :type "Float (single-precision)"))
  (bind (_velocity_x _velocity_y _velocity_z) (`KismetMathLibrary.BreakVector` (`MovementComponent.Velocity` (`self.CharacterMovement`))))
  (set `self.WillFallDown` (<= _velocity_z -1000.0)))

(event `ResetPosition`
  (`self.K2_SetActorLocation` (`self.BasePosition`))
  (`self.FallDown`)
  (bind _returnvalue (`GameplayStatics.GetActorOfClass` "/Game/Environment/BluePrints/BP_StartPoint.BP_StartPoint_C"))
  (`/Game/Environment/BluePrints/BP_StartPoint.Use` _returnvalue))

(event `EnhancedInput|/Game/Inputs/Actions/IA_Reset`
  (params (ActionValue :type Boolean) (ElapsedSeconds :type "Float (double-precision)") (TriggeredSeconds :type "Float (double-precision)") (InputAction :type "InputAction Object Reference" :default "/Game/Inputs/Actions/IA_Reset.IA_Reset"))
  (:`Triggered`
    (`self.ResetPosition`)))

(event `FallDown`
  (set `self.CanMove` false)
  (`|PlayMontage` (`self.Mesh`) "/Game/Characters/Robot/AM_FallDown.AM_FallDown"
    (:`OnCompleted`
      (`KismetSystemLibrary.Delay` 2.0)
      (set `self.CanMove` true))))

(fn `UserConstructionScript`)